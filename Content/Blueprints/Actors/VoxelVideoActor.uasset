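; VoxelVideoActor is an actor that displays voxel video at a world position, with audio placed at the same location.
; Construction feeds VoxelVideoSource into VoxelRender and sets the render and audio placement from the actor's transform, keeping only yaw, divided by 360.
; TransformToMarker repositions both the same way from a supplied marker transform.
; Play, Pause and Stop pass straight through to the video source.
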(event EventBeginPlay)

(event Collision|EventActorBeginOverlap
  (params (OtherActor :type Actor%20Object%20Reference)))

(event EventTick
  (params (DeltaSeconds :type Float%20%28single-precision%29)))

(fn ConstructionScript
  (bind _returnvalue (Transformation|GetActorTransform))
  (bind _voxelrender (Variables|Default|GetVoxelRender))
  (Variables|/Script/Voxels.VoxelRenderComponent|SetVoxelSource (Variables|Default|GetVoxelRender) (Variables|Default|GetVoxelVideoSource))
  (Class|VoxelRenderComponent|SetLocation _voxelrender (.location _returnvalue))
  (Class|VoxelRenderComponent|SetRotation _voxelrender (Math|Vector|MakeVector (/ (.Yaw (Math|Rotator|BreakRotator (.rotation _returnvalue))) 3.6e+02) 0.0 0.0))
  (Class|VoxelVideoSourceComponent|SetAudioLocation (Variables|Default|GetVoxelVideoSource) (.location _returnvalue)))

(fn Pause
  (Class|VoxelVideoSourceComponent|Pause (Variables|Default|GetVoxelVideoSource)))

(fn Play
  (Class|VoxelVideoSourceComponent|Play (Variables|Default|GetVoxelVideoSource)))

(fn Stop
  (Class|VoxelVideoSourceComponent|Stop (Variables|Default|GetVoxelVideoSource)))

(fn TransformtoMarker
  (params (MarkerTransform :type Transform))
  (bind _voxelrender (Variables|Default|GetVoxelRender))
  (Class|VoxelRenderComponent|SetLocation _voxelrender (.location MarkerTransform))
  (Class|VoxelRenderComponent|SetRotation _voxelrender (Math|Vector|MakeVector (/ (.Yaw (Math|Rotator|BreakRotator (.rotation MarkerTransform))) 3.6e+02) 0.0 0.0))
  (Class|VoxelVideoSourceComponent|SetAudioLocation (Variables|Default|GetVoxelVideoSource) (.location MarkerTransform)))